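; Bp_Caouch is a couch that tracks how soaked it gets from pee projectiles.
; Each ProjectilePisse that begins overlapping its Box adds one to NivPisse and prints the new level.
; Tick polls that level and, once it reaches the full threshold, sets CaouchPleinDPisse and prints a "full" message every frame.
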(event `self.ReceiveTick`
  (params (DeltaSeconds :type "Float (single-precision)"))
  (if (>= (`self.NivPisse`) 100.0)
    (`KismetSystemLibrary.PrintString` "Caouch Plein de pisse")
    (set `self.CaouchPleinDPisse` true)))

(event `self.Box.OnComponentBeginOverlap`
  (params (OverlappedComponent :type "PrimitiveComponent Object Reference") (OtherActor :type "Actor Object Reference") (OtherComp :type "PrimitiveComponent Object Reference") (OtherBodyIndex :type Integer) (bFromSweep :type Boolean) (SweepResult :type "HitResult Structure (by ref)"))
  (cast `/Game/Blueprint/AiBoss/ProjectilePisse` OtherActor)
  (bind _output_get (set `self.NivPisse` (+ (`self.NivPisse`) 1.0)))
  (`KismetSystemLibrary.PrintString` (`KismetStringLibrary.Conv_DoubleToString` _output_get) true true (struct :`G` 0.66 :`B` 1.0 :`A` 1.0) 1.0))

(fn `UserConstructionScript`)