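; Bp_Meuble is a furniture actor that the Bp_CelinePoulin character can grab and move.
; An overlap box tracks whether something is in range, disabling gravity and setting a physical material override on entry.
; Each Tick polls every Celine: while grabbing in range, the furniture attaches to her, loses cube collision and locks her rotation to LockRotationCeline.
; When not grabbing, it detaches, restoring collision and movement-oriented rotation.
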(event `self.BoxMiddle.OnComponentEndOverlap`
  (params (OverlappedComponent :type "PrimitiveComponent Object Reference") (OtherActor :type "Actor Object Reference") (OtherComp :type "PrimitiveComponent Object Reference") (OtherBodyIndex :type Integer))
  (set `self.isInBox` false))

(event `self.BoxMiddle.OnComponentBeginOverlap`
  (params (OverlappedComponent :type "PrimitiveComponent Object Reference") (OtherActor :type "Actor Object Reference") (OtherComp :type "PrimitiveComponent Object Reference") (OtherBodyIndex :type Integer) (bFromSweep :type Boolean) (SweepResult :type "HitResult Structure (by ref)"))
  ;[1 1 1] isCeline is in the Box?
  (set `self.isInBox` true)
  (`PrimitiveComponent.SetEnableGravity` (`self.BoxMiddle`) false)
  (`PrimitiveComponent.SetEnableGravity` (`self.Cube`) false)
  (`PrimitiveComponent.SetPhysMaterialOverride` (`self.Cube`) null))

(event `self.ReceiveTick`
  (params (DeltaSeconds :type "Float (single-precision)"))
  ;[1 1 1] Celine Grab
  (bind _outactors (`GameplayStatics.GetAllActorsOfClass` "/Game/Blueprint/Junk/Bp_CelinePoulin.Bp_CelinePoulin_C"))
  (for _array_element _outactors
    (if (`/Game/Blueprint/Junk/Bp_CelinePoulin.isGrab` _array_element)
      (if (`self.isInBox`)
        (`self.K2_AttachToActor` self _array_element "None" "KeepWorld" "KeepRelative" "KeepWorld" false)
        (`PrimitiveComponent.SetCollisionEnabled` (`self.Cube`) "NoCollision")
        (`self.K2_SetActorRotation` _array_element (`KismetMathLibrary.TransformRotation` (`self.LockRotationCeline`)) false)
        (bind _charactermovement (`Character.CharacterMovement` _array_element))
        (set `CharacterMovementComponent.bOrientRotationToMovement` false _charactermovement))
      (else
        ;[1 1 1] Celine lache
        (`self.K2_DetachFromActor` self "KeepWorld" "KeepWorld" "KeepWorld")
        (`PrimitiveComponent.SetCollisionEnabled` (`self.Cube`) "QueryAndPhysics")
        (set `CharacterMovementComponent.bOrientRotationToMovement` true _charactermovement)))))

(fn `UserConstructionScript`)